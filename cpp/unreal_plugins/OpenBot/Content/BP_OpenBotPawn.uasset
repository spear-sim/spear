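; BP_OpenBotPawn is a player-drivable vehicle pawn that forwards input to its vehicle movement component.
; The Throttle, Brake and Steering axis inputs pass straight through to the movement component's matching setters.
; Every tick it casts that component to OpenBotMovementComponent and prints its debug values.
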(event EventBeginPlay)

(event Collision|EventActorBeginOverlap
  (params (OtherActor :type Actor%20Object%20Reference)))

(event EventTick
  (params (DeltaSeconds :type Float%20%28single-precision%29))
  (bind _asopen_bot_movement_component (Utilities|Casting|CastToOpenBotMovementComponent (Variables|Default|GetVehicleMovementComponent)))
  (Class|OpenBotMovementComponent|PrintDebugValues _asopen_bot_movement_component))

(event Input|AxisEvents|InputAxisThrottle
  (params (AxisValue :type Float%20%28single-precision%29))
  (Class|ChaosVehicleMovementComponent|SetThrottleInput (Variables|Default|GetVehicleMovementComponent) AxisValue))

(event Input|AxisEvents|InputAxisBrake
  (params (AxisValue :type Float%20%28single-precision%29))
  (Class|ChaosVehicleMovementComponent|SetBrakeInput (Variables|Default|GetVehicleMovementComponent) AxisValue))

(event Input|AxisEvents|InputAxisSteering
  (params (AxisValue :type Float%20%28single-precision%29))
  (Class|ChaosVehicleMovementComponent|SetSteeringInput (Variables|Default|GetVehicleMovementComponent) AxisValue))

(fn ConstructionScript)
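; Light manager actor for the apartment scene that switches the lighting between day and night.
; Its construction script caches actors tagged Day and Night, lamp meshes tagged Lamp, and the HDRI backdrop.
; TurnOnOff toggles visibility of both light sets and the backdrop's geometry and skylight, recording day state from the day lights.
; It then creates dynamic instances of lamp Emissive materials, zeroing intensity by day and lighting them at night.
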(event EventBeginPlay)

(event Collision|EventActorBeginOverlap
  (params (OtherActor :type Actor%20Object%20Reference)))

(event EventTick
  (params (DeltaSeconds :type Float%20%28single-precision%29)))

(fn ConstructionScript
  (CallFunction|StoreLights))

(fn StoreLights
  (bind _outactors (Actor|GetAllActorswithTag "Day"))
  (Variables|Default|SetDayLights _outactors)
  (bind _outactors_2 (Actor|GetAllActorswithTag "Night"))
  (Variables|Default|SetNightLights _outactors_2)
  (bind _returnvalue (Actor|GetActorOfClass "/HDRIBackdrop/Blueprints/HDRIBackdrop.HDRIBackdrop_C"))
  (Variables|Default|SetHDRI _returnvalue)
  (bind _outactors_3 (Actor|GetAllActorsOfClasswithTag "/Script/Engine.StaticMeshActor" "Lamp"))
  (Variables|Default|SetLamps _outactors_3))

(fn TurnOn/Off
  (bind _hdri (Variables|Default|GetHDRI))
  (for _array_element (Variables|Default|GetDayLights)
    (Rendering|ToggleVisibility (Variables|/Script/Engine.Actor|GetRootComponent _array_element) false)
    (Variables|Default|SetDay/Night (Variables|/Script/Engine.SceneComponent|GetbVisible (Variables|/Script/Engine.Actor|GetRootComponent _array_element))))
  (Rendering|ToggleVisibility (Variables|/HDRIBackdrop/Blueprints/HDRIBackdrop.HDRIBackdrop_C|GetGeometry _hdri) false)
  (Rendering|ToggleVisibility (Variables|/HDRIBackdrop/Blueprints/HDRIBackdrop.HDRIBackdrop_C|GetSkylight _hdri) false)
  (for _array_element_2 (Variables|Default|GetNightLights)
    (Rendering|ToggleVisibility (Variables|/Script/Engine.Actor|GetRootComponent _array_element_2) false))
  (for _array_element_3 (Variables|Default|GetLamps)
    (bind _returnvalue (Rendering|Material|CreateDynamicMaterialInstance (Variables|/Script/Engine.StaticMeshActor|GetStaticMeshComponent _array_element_3) (Rendering|Material|GetMaterialIndex (Variables|/Script/Engine.StaticMeshActor|GetStaticMeshComponent _array_element_3) "Emissive") (Rendering|Material|GetMaterial (Variables|/Script/Engine.StaticMeshActor|GetStaticMeshComponent _array_element_3) (Rendering|Material|GetMaterialIndex (Variables|/Script/Engine.StaticMeshActor|GetStaticMeshComponent _array_element_3) "Emissive")) "None" :!class /Script/Engine.PrimitiveComponent))
    (if (Variables|Default|GetDay/Night)
      (Rendering|Material|SetScalarParameterValue _returnvalue "Em_Intensity" 0.0 :!class /Script/Engine.MaterialInstanceDynamic)
      (else
        (Rendering|Material|SetScalarParameterValue _returnvalue "Em_Intensity" 5e+01 :!class /Script/Engine.MaterialInstanceDynamic)))))
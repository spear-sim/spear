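; BP_OpenBotPawn is a drivable wheeled robot pawn that steers like a tank through Chaos vehicle physics.
; BeginPlay caches the Chaos wheeled movement component, which both input axes drive directly through per-wheel drive torque.
; Forward input applies equal torque to every wheel, while right input gives wheels 0/2 and 1/3 opposite torque.
; Both handlers set rather than sum torque, so they overwrite each other, and debug prints remain.
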(event EventTick
  (params (DeltaSeconds :type Float%20%28single-precision%29))
  ;[1 1 1] Movement component setup
)

(event EventBeginPlay
  ;[1 1 1] Movement component setup
  (bind _aschaos_wheeled_vehicle_movement_component (Utilities|Casting|CastToChaosWheeledVehicleMovementComponent (Variables|Default|GetVehicleMovementComponent)))
  (Variables|Default|SetChaos%20Wheeled%20Vehicle%20Movement%20Component _aschaos_wheeled_vehicle_movement_component)
  (Development|PrintText "InitHello"))

(event Input|AxisEvents|InputAxisBaseMoveForward
  (params (AxisValue :type Float%20%28single-precision%29))
  (CallFunction|MoveFoward AxisValue))

(event Input|AxisEvents|InputAxisBaseMoveRight
  (params (AxisValue :type Float%20%28single-precision%29))
  (CallFunction|MoveRight AxisValue)
  (Development|PrintText "Hello"))

(fn ConstructionScript)

(fn MoveFoward
  (params (val :type Float%20%28double-precision%29))
  (for _index (range 0 (- (Class|ChaosWheeledVehicleMovementComponent|GetNumWheels (Variables|Default|GetChaos%20Wheeled%20Vehicle%20Movement%20Component)) 1))
    (Class|ChaosWheeledVehicleMovementComponent|SetDriveTorque (Variables|Default|GetChaos%20Wheeled%20Vehicle%20Movement%20Component) val _index)))

(fn MoveRight
  (params (val :type Float%20%28double-precision%29))
  (bind _returnvalue (* val 1.0))
  (bind _returnvalue_2 (* val -1.0))
  (bind _chaos_wheeled_vehicle_movement_component (Variables|Default|GetChaos%20Wheeled%20Vehicle%20Movement%20Component))
  (Utilities|FlowControl|Sequence
    (:then_0
      (Class|ChaosWheeledVehicleMovementComponent|SetDriveTorque _chaos_wheeled_vehicle_movement_component _returnvalue))
    (:then_1
      (Class|ChaosWheeledVehicleMovementComponent|SetDriveTorque _chaos_wheeled_vehicle_movement_component _returnvalue 2))
    (:then_2
      (Class|ChaosWheeledVehicleMovementComponent|SetDriveTorque _chaos_wheeled_vehicle_movement_component _returnvalue_2 1))
    (:then_3
      (Class|ChaosWheeledVehicleMovementComponent|SetDriveTorque _chaos_wheeled_vehicle_movement_component _returnvalue_2 3)
      (Development|PrintText (Utilities|Text|ToText(Float) _returnvalue_2 "HalfToEven")))))